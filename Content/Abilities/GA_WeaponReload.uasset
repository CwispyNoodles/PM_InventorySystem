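; Gameplay ability for weapon reload that plays the reload montage on the character's first-person arms mesh.
; On activation it finds the avatar's EquipmentManagerComponent, gets the equipped item's ranged weapon modifier, and reads its reload animation.
; The ability ends right after starting the montage without waiting for completion, or immediately if any lookup or the character cast fails.
; It contains no ammo logic.
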(event `self.K2_ActivateAbility`
  (bind (_returnvalue_owneractor _returnvalue_avataractor) (break `GameplayAbilityActorInfo` (`self.GetActorInfo`)))
  (bind (_returnvalue_owneractor_2 _returnvalue_avataractor_2) (break `GameplayAbilityActorInfo` (`self.GetActorInfo`)))
  (bind _returnvalue (`Actor.GetComponentByClass` _returnvalue_avataractor "/Script/PM_InventorySystem.EquipmentManagerComponent"))
  (`/Engine/EditorBlueprintResources/StandardMacros.IsValid` _returnvalue
    (:`Is Valid`
      (bind _output_get (set `self.EquipmentManager` _returnvalue))
      (bind _equippeditem (`EquipmentManagerComponent.EquippedItem` _output_get))
      (`/Engine/EditorBlueprintResources/StandardMacros.IsValid` _equippeditem
        (:`Is Valid`
          (bind _output_get_2 (set `self.Equipped Item` _equippeditem))
          (bind (_bsuccess _returnvalue_2) (`ItemInstance.GetItemModifierByClass` _output_get_2 "/PM_InventorySystem/Items/Modifiers/B_DefaultRangedWeaponModifier.B_DefaultRangedWeaponModifier_C"))
          (if _bsuccess
            (set `self.RangedWeaponModifer` _returnvalue_2)
            (bind _asb_default_character (cast `/Game/ProjectFiles/Character/B_DefaultCharacter` _returnvalue_avataractor_2)
              (:`then`
                (`|PlayMontage` (`/Game/ProjectFiles/Character/B_DefaultCharacter.CharacterArms` _asb_default_character) (`RangedWeaponModifier.CharacterReloadAnimation` (`self.RangedWeaponModifer`))
                  (:`then`
                    (`self.K2_EndAbility`))))
              (:`CastFailed`
                (`self.K2_EndAbility`)))
            (else
              (`self.K2_EndAbility`))))
        (:`Is Not Valid`
          (`self.K2_EndAbility`))))
    (:`Is Not Valid`
      (`self.K2_EndAbility`))))