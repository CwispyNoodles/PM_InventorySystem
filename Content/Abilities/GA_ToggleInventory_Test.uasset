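; Test gameplay ability that toggles the player's inventory UI open or closed on activation, then ends.
; It gets the HUD component from the inventory subsystem; opening adds a widget created from the pawn's InventoryManagerComponent data.
; Opening sets Game and UI input with a visible cursor, while closing restores game-only input and look control.
; An unconnected older branch adds the widget straight to the viewport.
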(event `self.K2_ActivateAbility`
  (bind _returnvalue (`GameplayStatics.GetPlayerController` 0))
  (set `self.InventoryHUDComponent` (`InventorySubsystem.GetInventoryHUDComponent` (subsystem `InventorySubsystem`)))
  (if (`InventoryHUDComponent.IsInventoryOpen` (`self.InventoryHUDComponent`))
    (`InventoryHUDComponent.CloseInventory` (`self.InventoryHUDComponent`))
    (`WidgetBlueprintLibrary.SetInputMode_GameOnly` _returnvalue)
    (`Controller.SetIgnoreLookInput` _returnvalue false)
    (set `PlayerController.bShowMouseCursor` false (`GameplayStatics.GetPlayerController` 0))
    (`self.K2_EndAbility`)
    (else
      (bind (_bsuccess _returnvalue_2) (`InventoryHUDComponent.OpenInventory` (`self.InventoryHUDComponent`)))
      (if _bsuccess
        (bind _output_get (set `self.InventoryHUDWidget` _returnvalue_2))
        (`InventoryHUDWidget.AddChildWidget` _output_get (`InventoryData.CreateInventoryWidgetInstance` (`InventoryManagerComponent.GetInventoryData` (`Actor.GetComponentByClass` (`GameplayStatics.GetPlayerPawn` 0) "/Script/PM_InventorySystem.InventoryManagerComponent"))))
        (`WidgetBlueprintLibrary.SetInputMode_GameAndUIEx` (`GameplayStatics.GetPlayerController` 0) _output_get)
        (set `PlayerController.bShowMouseCursor` true (`GameplayStatics.GetPlayerController` 0))
        (`self.K2_EndAbility`)
        (else
          (`self.K2_EndAbility`))))))