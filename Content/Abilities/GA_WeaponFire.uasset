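; Weapon fire gameplay ability that fires one ranged shot through the associated item's ranged weapon modifier.
; Activation plays the modifier's fire montage on the character's arms, starts targeting and sets a rate-of-fire timer, apparently to end the ability.
; GetTargetData supplies the owner's camera location and forward vector for aiming.
; Returned target data passes the first hit's position, normal and surface to the modifier's Fire; gameplay cue code is unconnected.
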(event `self.OnRangedWeaponTargetDataReady`
  (params (TargetData :type "GameplayAbilityTargetDataHandle Structure (by ref)"))
  (bind _output_get (set `self.GCNParameter` (`GameplayCueFunctionLibrary.MakeGameplayCueParametersFromHitResult` (`AbilitySystemBlueprintLibrary.GetHitResultFromTargetData` TargetData))))
  (`KismetSystemLibrary.PrintString` "3")
  (bind (_normalizedmagnitude _rawmagnitude _effectcontext _matchedtagname _originaltag _aggregatedsourcetags _aggregatedtargettags _location _normal _instigator _effectcauser _sourceobject _physicalmaterial) (`AbilitySystemBlueprintLibrary.BreakGameplayCueParameters` _output_get))
  (`RangedWeaponModifier.Fire` (`.ReturnValue` (`ItemInstance.GetItemModifierByClass` (`self.GetAssociatedItem`) "/PM_InventorySystem/Items/Modifiers/B_DefaultRangedWeaponModifier.B_DefaultRangedWeaponModifier_C")) (`|MakeArray` _location) (`|MakeArray` _normal) (`|MakeArray` (select `bool` (`KismetSystemLibrary.IsValid` _physicalmaterial) :`false` "SurfaceType_Default" :`true` (`PhysicalMaterial.SurfaceType` _physicalmaterial)))))

(event `self.K2_ActivateAbility`
  (bind (_returnvalue_owneractor _returnvalue_avataractor) (break `GameplayAbilityActorInfo` (`self.GetActorInfo`)))
  (bind (_bsuccess _returnvalue) (`ItemInstance.GetItemModifierByClass` (`self.GetAssociatedItem`) "/PM_InventorySystem/Items/Modifiers/B_DefaultRangedWeaponModifier.B_DefaultRangedWeaponModifier_C"))
  (if _bsuccess
    (bind _output_get (set `self.Ranged Weapon Modifier` _returnvalue))
    (bind _asb_default_character (cast `/Game/ProjectFiles/Character/B_DefaultCharacter` _returnvalue_avataractor)
      (:`then`
        (`|PlayMontage` (`/Game/ProjectFiles/Character/B_DefaultCharacter.CharacterArms` _asb_default_character) (`RangedWeaponModifier.CharacterFireAnimation` (`self.Ranged Weapon Modifier`))
          (:`then`
            (`self.StartRangedWeaponTargeting`)
            (`KismetSystemLibrary.K2_SetTimerDelegate` (`|CreateDelegate` :!event `FireComplete`) (/ 60.0 (`RangedWeaponModifier.RateOfFire` _output_get))))))
      (:`CastFailed`
        (`self.K2_EndAbility`)))
    (else
      (`self.K2_EndAbility`))))

(event `FireComplete`
  (`self.K2_EndAbility`))

(fn `GetTargetData`
  (returns (ReturnValue :type "TargetData Structure"))
  (bind _asactor (cast `Actor` (`ItemInstance.GetOwner` (`self.GetAssociatedItem`))))
  (bind _returnvalue (`Actor.GetComponentByClass` _asactor "/Script/Engine.CameraComponent"))
  (`/Engine/EditorBlueprintResources/StandardMacros.IsValid` _returnvalue
    (:`Is Valid`
      (return (make `TargetData` (`SceneComponent.K2_GetComponentLocation` _returnvalue) (`SceneComponent.GetForwardVector` _returnvalue))))))