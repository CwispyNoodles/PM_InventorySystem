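; Gameplay ability that equips and unequips ranged weapons on the default character's arms mesh.
; It stays active, binding EquipmentManager delegates and turning equipment-slot gameplay events into active slot tags.
; Equip reads the slot item's RangedWeaponModifier, links its anim layer, attaches the spawned weapon and confirms after the montage.
; Unequip reverses this once its montage completes; interrupt and swap handlers are empty.
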(event `self.K2_ActivateAbility`
  (bind (_returnvalue_owneractor _returnvalue_avataractor) (break `GameplayAbilityActorInfo` (`self.GetActorInfo`)))
  (bind _asb_default_character (cast `/Game/ProjectFiles/Character/B_DefaultCharacter` _returnvalue_avataractor))
  (set `self.OwnerSkeletalMesh` (`/Game/ProjectFiles/Character/B_DefaultCharacter.CharacterArms` _asb_default_character))
  (set `self.EquipmentManager` (`/Game/ProjectFiles/Character/B_DefaultCharacter.EquipmentManager` _asb_default_character))
  (set `self.InventoryManager` (`/Game/ProjectFiles/Character/B_DefaultCharacter.InventoryManager` _asb_default_character))
  (if (and (`KismetSystemLibrary.IsValid` (`self.EquipmentManager`)) (`KismetSystemLibrary.IsValid` (`self.InventoryManager`)))
    (`|ExecutionSequence`
      (:`then_0`
        (add `EquipmentManagerComponent.OnEquipDelegate` (`self.EquipmentManager`) (`|CreateDelegate` :!event `OnEquipEvent`)))
      (:`then_1`
        (add `EquipmentManagerComponent.OnUnequipDelegate` (`self.EquipmentManager`) (`|CreateDelegate` :!event `OnUnequipEvent`)))
      (:`then_2`
        (add `EquipmentManagerComponent.OnInterruptDelegate` (`self.EquipmentManager`) (`|CreateDelegate` :!event `OnInterruptEvent`)))
      (:`then_3`
        (add `EquipmentManagerComponent.OnSwapDelegate` (`self.EquipmentManager`) (`|CreateDelegate` :!event `OnSwapEvent`)))
      (:`then_4`
        ;[1 1 1] Permanent Active-Listener for EquipmentSlot Events
        (bind (_asynctaskproxy _payload) (`AbilityTask_WaitGameplayEvent.WaitGameplayEvent` (struct :`TagName` "InputTag.Ability.EquipmentSlot") null)
          (:`EventReceived`
            (`EquipmentManagerComponent.SetActiveEquipmentTag` (`self.EquipmentManager`) (`|GetArrayItem` (`BlueprintGameplayTagLibrary.BreakGameplayTagContainer` (`.InstigatorTags` (break `GameplayEventData` _payload)))))))))
    (else
      (`self.K2_EndAbility`))))

(event `OnEquipEvent`
  (bind _returnvalue (`EquipmentManagerComponent.GetActiveEquipmentTag` (`self.EquipmentManager`)))
  (bind (_bsuccess _returnvalue_2) (`ItemInstance.GetItemModifierByClass` (`self.EquippedSlotItem`) "/Script/PM_InventorySystem.RangedWeaponModifier"))
  (bind (_bsuccess_2 _returnvalue_3) (`InventoryManagerComponent.GetInventorySlotDataByTag` (`self.InventoryManager`) _returnvalue))
  (if _bsuccess_2
    (bind _output_get (set `self.EquippedSlotData` _returnvalue_3))
    (bind _returnvalue_4 (`InventorySlotData.GetSlotItem` _output_get))
    (`/Engine/EditorBlueprintResources/StandardMacros.IsValid` _returnvalue_4
      (:`Is Valid`
        (set `self.EquippedSlotItem` _returnvalue_4)
        (if _bsuccess
          (bind _output_get_2 (set `self.EquippedRangedModifier` _returnvalue_2))
          (bind (_value _returnvalue_5) (`BlueprintMapLibrary.Map_Find` (`WeaponModifier.CharacterEquipAnimations` _output_get_2) (`EquipmentManagerComponent.GetActiveEquipmentTag` (`self.EquipmentManager`))))
          (if _returnvalue_5
            (set `self.LastActiveEquipmentSlot` _returnvalue)
            (`SkeletalMeshComponent.LinkAnimClassLayers` (`self.OwnerSkeletalMesh`) (`WeaponModifier.EquipmentAnimationLayer` (`self.EquippedRangedModifier`)))
            (bind _returnvalue_6 (`EquipmentModifier.SpawnEquipmentActor` :`self` (`self.EquippedRangedModifier`)))
            (bind _output_get_3 (set `self.SpawnedItem` _returnvalue_6))
            (`Actor.K2_AttachToComponent` _output_get_3 (`self.OwnerSkeletalMesh`) "ik_hand_gun" "SnapToTarget" "SnapToTarget" "SnapToTarget" true)
            (`|PlayMontage` (`self.OwnerSkeletalMesh`) (`.EquipAnimation` (break `WeaponAnimations` _value))
              (:`OnCompleted`
                (`EquipmentManagerComponent.EquipItem` (`self.EquipmentManager`) (`self.EquippedSlotItem`))))))))))

(event `OnInterruptEvent`)

(event `OnSwapEvent`)

(event `OnUnequipEvent`
  (bind (_bsuccess _returnvalue) (`InventoryManagerComponent.GetInventorySlotDataByTag` (`self.InventoryManager`) (`self.LastActiveEquipmentSlot`)))
  (bind (_bsuccess_2 _returnvalue_2) (`ItemInstance.GetItemModifierByClass` (`self.EquippedSlotItem`) "/Script/PM_InventorySystem.RangedWeaponModifier"))
  (if _bsuccess
    (bind _output_get (set `self.EquippedSlotData` _returnvalue))
    (bind _returnvalue_3 (`InventorySlotData.GetSlotItem` _output_get))
    (`/Engine/EditorBlueprintResources/StandardMacros.IsValid` _returnvalue_3
      (:`Is Valid`
        (set `self.EquippedSlotItem` _returnvalue_3)
        (if _bsuccess_2
          (bind _output_get_2 (set `self.EquippedRangedModifier` _returnvalue_2))
          (bind (_value _returnvalue_4) (`BlueprintMapLibrary.Map_Find` (`WeaponModifier.CharacterEquipAnimations` _output_get_2) (`self.LastActiveEquipmentSlot`)))
          (if _returnvalue_4
            (`|PlayMontage` (`self.OwnerSkeletalMesh`) (`.UnequipAnimation` (break `WeaponAnimations` _value))
              (:`OnCompleted`
                (`SkeletalMeshComponent.LinkAnimClassLayers` (`self.OwnerSkeletalMesh`) (`EquipmentManagerComponent.DefaultAnimationLayer` (`self.EquipmentManager`)))
                (`Actor.K2_DestroyActor` (`self.SpawnedItem`))
                (`EquipmentManagerComponent.UnequipItem` (`self.EquipmentManager`))))))))))